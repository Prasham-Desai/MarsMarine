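; BP_MissionAreaVolume is a mission boundary that kills the player if they stay outside it too long.
; Begin and end overlap events set IsInBounds on any overlapping BP_Marine, clearing the KillPlayer timer on entry and starting it with ReturnToAreaTimer on exit.
; When the timer fires, KillPlayer applies MaxHealth damage to player character 0, regardless of which marine left, then clears the timer.
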(event `self.ReceiveActorBeginOverlap`
  (params (OtherActor :type "Actor Object Reference"))
  ;[0 0.15 0.02286 0.5] Check Player Bounds
  (bind _asbp_marine (cast `/Game/Blueprints/Pawns/BP_Marine` OtherActor))
  (set `/Game/Blueprints/Pawns/BP_Marine.IsInBounds` true _asbp_marine)
  (`KismetSystemLibrary.K2_ClearTimer` null "KillPlayer"))

(event `self.ReceiveActorEndOverlap`
  (params (OtherActor :type "Actor Object Reference"))
  ;[0 0.15 0.02286 0.5] Check Player Bounds
  (bind _asbp_marine (cast `/Game/Blueprints/Pawns/BP_Marine` OtherActor))
  (set `/Game/Blueprints/Pawns/BP_Marine.IsInBounds` false _asbp_marine)
  (`KismetSystemLibrary.K2_SetTimer` null "KillPlayer" (`self.ReturnToAreaTimer`)))

(fn `KillPlayer`
  (bind _returnvalue (`GameplayStatics.GetPlayerCharacter` 0))
  (bind _asbp_marine (cast `/Game/Blueprints/Pawns/BP_Marine` _returnvalue))
  (`GameplayStatics.ApplyDamage` _returnvalue (`/Game/Blueprints/Pawns/BP_Marine.MaxHealth` _asbp_marine))
  (`KismetSystemLibrary.K2_ClearTimer` null "KillPlayer"))

(fn `UserConstructionScript`)