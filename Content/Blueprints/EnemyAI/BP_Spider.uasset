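; Spider enemy character that chases the player marine, attacks in melee range and dies from damage.
; A repeating AIMoveTo loop drives pursuit, while Tick checks range and player state, freezing movement during the attack montage.
; Death disables movement and collision, credits the marine's kill, notifies BP_GameMode, then destroys the actor after a delay.
; DamagePlayer and SetSpiderSpeed are helpers with no callers in this Blueprint.
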(event `self.ReceiveBeginPlay`
  ;[0.02713 0.0176 0.15 0.5] Locomotion
  (if (`self.IsSpiderAlive`) :!label _label
    (`|AIMoveTo` self (0.0 0.0 0.0) (`GameplayStatics.GetPlayerCharacter` 0)
      (:`OnSuccess`
        _)
      (:`OnFail`
        _))
    (`KismetSystemLibrary.Delay` 0.2)
    (goto _label)))

(event `self.ReceiveTick`
  (params (DeltaSeconds :type "Float (single-precision)"))
  ;[0.15 2.3e-05 0.006045 0.5] Attack
  (if (and (`self.CheckAttackValidity`) (`self.IsSpiderAlive`))
    (`self.DeactivateMovement`)
    (`|PlayMontage` (`self.Mesh`) "/Game/Characters/Enemy_Great_Spider/Animations/AlienAttack.AlienAttack"
      (:`OnCompleted`
        (`self.ActivateMovement`)))))

(event `self.ReceiveAnyDamage`
  (params (Damage :type "Float (single-precision)") (DamageType :type "DamageType Object Reference") (InstigatedBy :type "Controller Object Reference") (DamageCauser :type "Actor Object Reference"))
  ;[0.15 0 0.145 0.5] Take Damage
  (if (`self.IsSpiderAlive`)
    (bind _spiderhealthafterdamage (`self.DecreasSpiderHealth` Damage))
    (if (<= _spiderhealthafterdamage 0.0)
      (`self.KillSpider`)
      (`KismetSystemLibrary.Delay` 3.0)
      (`self.K2_DestroyActor`))))

(fn `ActivateMovement`
  (`ActorComponent.Activate` (`self.CharacterMovement`) false))

(fn `CheckAttackValidity`
  (returns (ReturnValue :type Boolean))
  (bind _asbp_marine (cast `/Game/Blueprints/Pawns/BP_Marine` (`GameplayStatics.GetPlayerCharacter` 0)))
  (return (and (`self.IsWithinAttackRange`) (not (`self.IsAttacking`)) (not (`/Game/Blueprints/Pawns/BP_Marine.IsPlayerDead` _asbp_marine)))))

(fn `DamagePlayer`
  (`GameplayStatics.ApplyDamage` (`GameplayStatics.GetPlayerCharacter` 0) (`self.SpiderDamage`)))

(fn `DeactivateMovement`
  (bind _charactermovement (`self.CharacterMovement`))
  (`MovementComponent.StopMovementImmediately` _charactermovement)
  (`ActorComponent.Deactivate` _charactermovement))

(fn `DecreasSpiderHealth`
  (params (B :type "Float (double-precision)"))
  (returns (SpiderHealthAfterDamage :type "Float (double-precision)"))
  (bind _output_get (set `self.SpiderHealth` (- (`self.SpiderHealth`) B)))
  (return _output_get))

(fn `IsAttacking`
  (returns (IsAttacking :type Boolean))
  (return (`AnimInstance.Montage_IsPlaying` (`SkeletalMeshComponent.GetAnimInstance` (`self.Mesh`)) "/Game/Characters/Enemy_Great_Spider/Animations/AlienAttack.AlienAttack")))

(fn `IsSpiderAlive`
  (returns (IsAlive :type Boolean))
  (return (not (`self.IsSpiderDead`))))

(fn `IsWithinAttackRange`
  (returns (IsWithinAttackRange :type Boolean))
  (return (<= (`self.GetDistanceTo` (`GameplayStatics.GetPlayerCharacter` 0)) (`self.AttackRange`))))

(fn `KillSpider`
  (set `self.IsSpiderDead` true)
  (`self.DeactivateMovement`)
  (`self.SetActorEnableCollision` false)
  (bind _asbp_marine (cast `/Game/Blueprints/Pawns/BP_Marine` (`GameplayStatics.GetPlayerCharacter` 0)))
  (`/Game/Blueprints/Pawns/BP_Marine.Increase Kills` _asbp_marine)
  (bind _asbp_game_mode (cast `/Game/Blueprints/GameModes/BP_GameMode` (`GameplayStatics.GetGameMode`)))
  (`/Game/Blueprints/GameModes/BP_GameMode.RegisterSpiderDeath` _asbp_game_mode self))

(fn `SetSpiderSpeed`
  (params (SpeedIncrease :type "Float (double-precision)"))
  (bind _charactermovement (`self.CharacterMovement`))
  (set `CharacterMovementComponent.MaxWalkSpeed` (+ SpeedIncrease (`CharacterMovementComponent.MaxWalkSpeed` _charactermovement)) _charactermovement))

(fn `UserConstructionScript`)