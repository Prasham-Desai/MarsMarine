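; BP_HealthPickup is a health pickup that heals the player's marine on overlap.
; When the overlapping actor is the player character cast to BP_Marine and its health is not full, it adds HealthValue through AddHealth.
; It then plays HealSound at its location and destroys itself, so a marine at full health leaves the pickup in place.
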(event `self.ReceiveActorBeginOverlap`
  (params (OtherActor :type "Actor Object Reference"))
  (bind _asbp_marine (cast `/Game/Blueprints/Pawns/BP_Marine` (`GameplayStatics.GetPlayerCharacter` 0)))
  (set `self.Marine` _asbp_marine)
  (if (== _asbp_marine OtherActor)
    (if (not (`/Game/Blueprints/Pawns/BP_Marine.IsHealthFull` (`self.Marine`)))
      (`/Game/Blueprints/Pawns/BP_Marine.AddHealth` (`self.Marine`) (`self.HealthValue`))
      (`GameplayStatics.PlaySoundAtLocation` "/Game/Sounds/HealSound.HealSound" (`self.K2_GetActorLocation` self) (struct) 1.0 1.0 0.0 null null null null)
      (`self.K2_DestroyActor` self))))

(fn `UserConstructionScript`)