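; Game mode that runs endless waves of spiders, starting shortly after BeginPlay.
; Each wave sets a spawn count from difficulty variables, then a looping timer spawns spiders at random TargetPoints until that count runs out.
; Spider health and speed scale in steps with the wave number.
; RegisterSpiderDeath starts the next wave once all are spawned and dead; EndWave can also start one after a delay.
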(event `self.ReceiveBeginPlay`
  ;[0 0.1347 0.15 0.5] Setup Wave
  (`KismetSystemLibrary.Delay` 1.0)
  (`self.SetupNewWave`))

(event `SpawnWave`
  ;[0.15 0.01931 0.005174 0.5] Spawn Spider
  (`self.SpawnSpider`))

(event `EndWave`
  ;[0 0.1135 0.15 0.5] Setup New Wave
  (`KismetSystemLibrary.Delay` 2.0)
  (`self.SetupNewWave`))

(fn `GetRandomSpawnPoint`
  (returns (SpawnPoint :type "TargetPoint Object Reference"))
  (bind _outactors (`GameplayStatics.GetAllActorsOfClass` "/Script/Engine.TargetPoint"))
  (return (`|GetArrayItem` _outactors (`KismetMathLibrary.RandomInteger` (`KismetArrayLibrary.Array_Length` _outactors)))))

(fn `IncreaseSpeedPerNRounds`
  (params (Spider :type "/Game/Blueprints/EnemyAI/BP_Spider Object Reference"))
  (`/Game/Blueprints/EnemyAI/BP_Spider.SetSpiderSpeed` Spider (`KismetMathLibrary.Conv_IntToDouble` (* (/ (- (`self.CurrentWave`) 1) (`self.DifficultyIncreasePer`)) (`self.SpeedIncrease`)))))

(fn `IncreaseSpiderHealthAndSpeed`
  (params (Spider :type "/Game/Blueprints/EnemyAI/BP_Spider Object Reference"))
  (returns (IncreasedSpiderHealth :type "Float (double-precision)"))
  (`self.IncreaseSpeedPerNRounds` Spider)
  (bind _maxhealth (`self.IncreaseSpiderHealthPerNRounds` Spider))
  (return _maxhealth))

(fn `IncreaseSpiderHealthPerNRounds`
  (params (Spider :type "/Game/Blueprints/EnemyAI/BP_Spider Object Reference"))
  (returns (MaxHealth :type "Float (double-precision)"))
  (return (+ (`/Game/Blueprints/EnemyAI/BP_Spider.SpiderHealth` Spider) (* (/ (- (`self.CurrentWave`) 1) (`self.DifficultyIncreasePer`)) (`self.HealthBonus`)))))

(fn `IncreaseWaveDifficulty`
  (bind _output_get (set `self.WaveDifficulty` (`KismetMathLibrary.Round` (* (`self.SpiderCountIncreaseAmt`) (`self.DifficultyMultiplier`)))))
  (set `self.SpiderSpawnRemaining` _output_get))

(fn `RegisterSpiderDeath`
  (params (DeadSpider :type "/Game/Blueprints/EnemyAI/BP_Spider Object Reference (by ref)"))
  (`KismetArrayLibrary.Array_RemoveItem` (`self.Spiders`) DeadSpider)
  (if (and (== (`self.SpiderSpawnRemaining`) 0) (== (`KismetArrayLibrary.Array_Length` (`self.Spiders`)) 0))
    (`self.SetupNewWave`)))

(fn `SetupNewWave`
  (`/Engine/EditorBlueprintResources/StandardMacros.IncrementInt` (`self.CurrentWave`)
    (:`  `
      (`self.IncreaseWaveDifficulty`)
      (`KismetSystemLibrary.K2_SetTimer` null "SpawnWave" (`self.SpawnFrequency`) true))))

(fn `SpawnSpider`
  (bind _spiderspawnremaining (`self.SpiderSpawnRemaining`))
  (bind _spawnpoint (`self.GetRandomSpawnPoint`))
  (`/Engine/EditorBlueprintResources/StandardMacros.IsValid` _spawnpoint
    (:`Is Valid`
      (bind _returnvalue (`|SpawnActorFromClass` "/Game/Blueprints/EnemyAI/BP_Spider.BP_Spider_C" (`self.GetTransform` _spawnpoint) "Undefined" "MultiplyWithRoot" null null))
      (bind _increasedspiderhealth (`self.IncreaseSpiderHealthAndSpeed` _returnvalue))
      (set `/Game/Blueprints/EnemyAI/BP_Spider.SpiderHealth` _increasedspiderhealth _returnvalue)
      (`/Engine/EditorBlueprintResources/StandardMacros.IsValid` _returnvalue
        (:`Is Valid`
          (`KismetArrayLibrary.Array_Add` (`self.Spiders`) _returnvalue)
          (`/Engine/EditorBlueprintResources/StandardMacros.DecrementInt` _spiderspawnremaining
            (:`  `
              (if (== _spiderspawnremaining 0)
                (`KismetSystemLibrary.K2_ClearTimer` null "SpawnWave")))))))))

(fn `UserConstructionScript`)