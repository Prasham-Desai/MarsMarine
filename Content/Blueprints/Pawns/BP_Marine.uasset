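; Player-controlled marine pawn for a twin-stick shooter, with world-axis movement, aiming, automatic rifle fire, health and a kill counter.
; Tick aims through control rotation, smoothly turning toward the mouse cursor's trace hit or snapping to the thumbstick, based on the last key's device.
; Firing runs looping hitscan traces from the muzzle socket on a timer, with flash and sound.
; Damage lowers health; death gates input, aim and firing.
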(event `self.ReceiveBeginPlay`
  ;[0.15 0.1204 0.02908 0.5] Setting Mapping Context and Cursor on BeginPlay Event
  (`EnhancedInputSubsystemInterface.AddMappingContext` (pcsubsystem `EnhancedInputLocalPlayerSubsystem` (`GameplayStatics.GetPlayerController` 0)) "/Game/Input/IMC_Context.IMC_Context" 0 (struct))
  (set `PlayerController.bShowMouseCursor` true (`GameplayStatics.GetPlayerController` 0))
  (`ActorComponent.Deactivate` (`self.Muzzle Flash`))
  (bind _returnvalue (`|CreateWidget` "/Game/UI/WBP_HUD.WBP_HUD_C" null self))
  (`UserWidget.AddToViewport` _returnvalue 0))

(event `EnhancedInput|/Game/Input/IA_FWBW`
  (params (ActionValue :type "Float (double-precision)") (ElapsedSeconds :type "Float (double-precision)") (TriggeredSeconds :type "Float (double-precision)") (InputAction :type "InputAction Object Reference" :default "/Game/Input/IA_FWBW.IA_FWBW"))
  ;[0.01399 0.15 0 0.5] Character Movement
  (:`Triggered`
    (if (`self.IsAlive`)
      (`self.AddMovementInput` (1.0 0.0 0.0) ActionValue))))

(event `self.ReceiveAnyDamage`
  (params (Damage :type "Float (single-precision)") (DamageType :type "DamageType Object Reference") (InstigatedBy :type "Controller Object Reference") (DamageCauser :type "Actor Object Reference"))
  ;[0.15 0.002054 0.1013 0.5] Take Damage
  (if (`self.IsAlive`)
    (bind _health (`self.DecreasePlayerHealth` Damage))
    (bind _output_get (set `self.IsPlayerDead` (<= _health 0.0)))
    (if _output_get
      (`self.StopFiringWeapon`)
      (`AudioComponent.Stop` (`self.WeaponFireSound`))
      (else
        (`GameplayStatics.PlaySound2D` null 1.0 1.0 0.0 null null)))))

(event `EnhancedInput|/Game/Input/IA_LR`
  (params (ActionValue :type "Float (double-precision)") (ElapsedSeconds :type "Float (double-precision)") (TriggeredSeconds :type "Float (double-precision)") (InputAction :type "InputAction Object Reference" :default "/Game/Input/IA_LR.IA_LR"))
  ;[0.01399 0.15 0 0.5] Character Movement
  (:`Triggered`
    (if (`self.IsAlive`)
      (`self.AddMovementInput` (0.0 1.0 0.0) ActionValue))))

(event `Key|AnyKey`
  (params (Key :type "Key Structure"))
  ;[0 0.15 0.1281 0.5] Player Aim
  (:`Pressed`
    (set `self.IsGamePadActive` (`KismetInputLibrary.Key_IsGamepadKey` Key))))

(event `EnhancedInput|/Game/Input/IA_Fire`
  (params (ActionValue :type Boolean) (ElapsedSeconds :type "Float (double-precision)") (TriggeredSeconds :type "Float (double-precision)") (InputAction :type "InputAction Object Reference" :default "/Game/Input/IA_Fire.IA_Fire"))
  ;[0.15 0.02188 0 0.5] Weapon Firing
  (:`Started`
    (`self.StartFiringWeapon`)
    (`self.WeaponTrace`))
  (:`Completed`
    (`self.StopFiringWeapon`)))

(event `self.ReceiveTick`
  (params (DeltaSeconds :type "Float (single-precision)"))
  ;[0 0.15 0.1281 0.5] Player Aim
  (if (`self.IsAlive`)
    (`self.UpdatePlayerAim`)))

(fn `CalculateRotationMouse`
  (params (Target :type "Vector Structure (by ref)"))
  (returns (ReturnValue_Yaw :type "Float (single-precision)"))
  (bind (_returnvalue_roll _returnvalue_pitch _returnvalue_yaw) (`KismetMathLibrary.BreakRotator` (`KismetMathLibrary.RInterpTo` (`Controller.GetControlRotation` (`GameplayStatics.GetPlayerController` 0)) (`KismetMathLibrary.FindLookAtRotation` (`self.K2_GetActorLocation`) Target) (`GameplayStatics.GetWorldDeltaSeconds`) (`self.MouseSmoothingSpeed`))))
  (return _returnvalue_yaw))

(fn `DecreasePlayerHealth`
  (params (B :type "Float (double-precision)"))
  (returns (Health :type "Float (double-precision)"))
  (bind _output_get (set `self.PlayerHealth` (- (`self.PlayerHealth`) B)))
  (return _output_get))

(fn `GetThumStickAimDir`
  (returns (ReturnValue :type "Rotator Structure"))
  (bind (_returnvalue_x _returnvalue_y) (`KismetMathLibrary.BreakVector2D` (`|GetInputActionValue`)))
  (return (`KismetMathLibrary.MakeRotator` 0.0 0.0 (`KismetMathLibrary.DegAtan2` _returnvalue_x _returnvalue_y))))

(fn `GetWeaponTraceEndLocation`
  (returns (EndLocation :type "Vector Structure"))
  (return (+ (`self.GetWeaponTraceStartLocation`) (* (`KismetMathLibrary.GetForwardVector` (`self.GetControlRotation`)) (`self.WeaponRange`)))))

(fn `GetWeaponTraceStartLocation`
  (returns (ReturnValue :type "Vector Structure"))
  (return (`SceneComponent.GetSocketLocation` (`self.Rifle`) "MuzzleFlashSocket")))

(fn `Increase Kills`
  (`/Engine/EditorBlueprintResources/StandardMacros.IncrementInt` (`self.EnemiesKilled`)))

(fn `IsAlive`
  (returns (IsPlayerAlive :type Boolean))
  (return (not (`self.IsPlayerDead`))))

(fn `IsThumbStickBeingUsed`
  (returns (ReturnValue :type Boolean))
  (return (> (`KismetMathLibrary.VSize2D` (`|GetInputActionValue`)) 0.0)))

(fn `LineTraceMouse`
  (returns (OutHit_Location :type "Vector Structure"))
  (bind _returnvalue (`GameplayStatics.GetPlayerController` 0))
  (bind (_locationx _locationy) (`PlayerController.GetMousePosition` _returnvalue))
  (bind (_worldposition _worlddirection) (`GameplayStatics.DeprojectScreenToWorld` _returnvalue (`KismetMathLibrary.MakeVector2D` _locationx _locationy)))
  (bind _outhit (`KismetSystemLibrary.LineTraceSingle` _worldposition (+ _worldposition (* _worlddirection 3000.0)) "TraceTypeQuery1"))
  (return (`.Location` (`GameplayStatics.BreakHitResult` _outhit))))

(fn `StartFiringWeapon`
  (if (`self.IsAlive`)
    (`ActorComponent.Activate` (`self.Muzzle Flash`) false)
    (bind _returnvalue (`GameplayStatics.SpawnSound2D` "/Game/Sounds/Weapon_AssaultRifle/Stereo/AssautRifleShot.AssautRifleShot" 1.0 1.0 0.0 null false false))
    (set `self.WeaponFireSound` _returnvalue)
    (`KismetSystemLibrary.K2_SetTimer` null "WeaponTrace" (`self.FireRate`) true)))

(fn `StopFiringWeapon`
  (bind _muzzle_flash (`self.Muzzle Flash`))
  (`ActorComponent.Deactivate` _muzzle_flash)
  (`KismetSystemLibrary.K2_ClearTimer` null "WeaponTrace")
  (if (`self.IsAlive`)
    (`GameplayStatics.PlaySoundAtLocation` "/Game/Sounds/Weapon_AssaultRifle/Stereo/StopFiring.StopFiring" (`SceneComponent.K2_GetComponentLocation` _muzzle_flash) (struct) 1.0 1.0 0.0 null null null null)
    (`AudioComponent.Stop` (`self.WeaponFireSound`))))

(fn `UpadateGamePadAim`
  (if (`self.IsThumbStickBeingUsed`)
    (`Controller.SetControlRotation` (`GameplayStatics.GetPlayerController` 0) (`self.GetThumStickAimDir`))))

(fn `UpdateMouseAim`
  (bind _outhit_location (`self.LineTraceMouse`))
  (`Controller.SetControlRotation` (`GameplayStatics.GetPlayerController` 0) (`KismetMathLibrary.MakeRotator` 0.0 0.0 (`self.CalculateRotationMouse` _outhit_location))))

(fn `UpdatePlayerAim`
  (if (`self.IsGamePadActive`)
    (`self.UpadateGamePadAim`)
    (else
      (`self.UpdateMouseAim`))))

(fn `UserConstructionScript`)

(fn `WeaponTrace`
  (if (`self.IsAlive`)
    (bind _outhit (`KismetSystemLibrary.LineTraceSingle` (`self.GetWeaponTraceStartLocation`) (`self.GetWeaponTraceEndLocation`) "TraceTypeQuery1"))
    (bind (_bblockinghit _binitialoverlap _time _distance _location _impactpoint _normal _impactnormal _physmat _hitactor) (`GameplayStatics.BreakHitResult` _outhit))
    (if _bblockinghit
      (`GameplayStatics.ApplyDamage` _hitactor (`self.BulletDamage`)))))